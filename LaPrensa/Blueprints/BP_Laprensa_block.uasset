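; BP_Laprensa_block is a press block trap that damages what it hits.
; When the third-person character enters TriggerZone while IsUnlocked is set, DropTimeLine plays from the start.
; BlockMesh hits apply fixed damage and print a debug message.
; The timeline-driven movement, indicator-light interface calls and state reset are unwired, and BeginPlay sets BlockMesh to None.
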(event `self.ReceiveBeginPlay`
  (bind _output_get (set `self.BlockMesh` null)))

(event `self.TriggerZone.OnComponentBeginOverlap`
  (params (OverlappedComponent :type "PrimitiveComponent Object Reference") (OtherActor :type "Actor Object Reference") (OtherComp :type "PrimitiveComponent Object Reference") (OtherBodyIndex :type Integer) (bFromSweep :type Boolean) (SweepResult :type "HitResult Structure (by ref)"))
  (cast `/Game/ThirdPerson/Blueprints/BP_ThirdPersonCharacter` OtherActor)
  (if (`self.bIsUnlocked`)
    (`TimelineComponent.PlayFromStart` (`self.DropTimeLine`))))

(event `self.BlockMesh.OnComponentHit`
  (params (HitComponent :type "PrimitiveComponent Object Reference") (OtherActor :type "Actor Object Reference") (OtherComp :type "PrimitiveComponent Object Reference") (NormalImpulse :type "Vector Structure") (Hit :type "HitResult Structure (by ref)"))
  (`GameplayStatics.ApplyDamage` OtherActor 50.0)
  (`KismetSystemLibrary.PrintString` "Impacto Detectado"))

(fn `UserConstructionScript`)